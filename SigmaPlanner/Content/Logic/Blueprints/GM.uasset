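; GM is a game-logic Blueprint that tracks whether play is in a planning or simulation state and creates preview actors for placeable classes.
; On BeginPlay it enters planning, then spawns one actor per Placeables entry in a rotated row below the world origin, storing each in PlaceablePreviews.
; ToggleState flips between the two states through their switch events, which only set State, and returns the new value.
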(event Custom|SwitchToPlanning
  (Variables|Default|SetState "NewEnumerator0"))

(event Custom|SwitchToSimulation
  (Variables|Default|SetState "NewEnumerator1"))

(event Custom|SpawnPlaceablePreviews
  (for (_array_element _array_index) (Variables|Default|GetPlaceables)
    (bind _returnvalue (Game|SpawnActorfromClass _array_element (Math|Transform|MakeTransform (Math|Vector|MakeVector (* _array_index (Variables|Default|GetPlaceablePreviewShift)) 0.0 -1e+03) "0, 0,-90.000000") "AlwaysSpawn" 0 0))
    (Utilities|Array|Add (Variables|Default|GetPlaceablePreviews) _returnvalue)))

(event EventBeginPlay
  (CallFunction|SwitchtoPlanning)
  (CallFunction|SpawnPlaceablePreviews))

(fn ConstructionScript)

(fn ToggleState
  (if (Utilities|Enum|Equal(Enum) (Variables|Default|GetState) "NewEnumerator0")
    (CallFunction|SwitchtoSimulation)
    (else
      (CallFunction|SwitchtoPlanning)))
  (return (Variables|Default|GetState)))