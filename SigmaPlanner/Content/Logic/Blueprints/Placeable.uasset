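; Base actor for objects placed in the world, with a scene capture that renders only the actor itself.
; Place spawns a copy at its transform and registers it in the game mode's Placed list.
; Tick toggles Snap components by matching AllowedComponents to ShowSnapsFor, so the last array entry decides visibility.
; Highlight and Unhighlight assign new dynamic materials to GetHighlightables results, which are empty here.
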(event Custom|Place
  (bind _returnvalue (Game|SpawnActorfromClass (Utilities|GetClass self) (Transformation|GetWorldTransform (Variables|Default|GetDefaultSceneRoot)) "AlwaysSpawn" 0 0))
  (Utilities|Array|Add (Variables|/Game/Logic/Blueprints/GM.GM_C|GetPlaced (Utilities|GetGM)) _returnvalue))

(event Custom|Highlight
  (if (not (Variables|Default|GetHighlighted))
    (Variables|Default|SetHighlighted true)
    (for _array_element (CallFunction|GetHighlightables)
      (bind _returnvalue (Rendering|Material|GetBaseMaterial (Rendering|Material|GetMaterial _array_element 0)))
      (bind _returnvalue_2 (Rendering|Material|CreateDynamicMaterialInstance _returnvalue "None" :!class /Script/Engine.KismetMaterialLibrary))
      (Rendering|Material|SetScalarParameterValue _returnvalue_2 "Highlight" 1.0 :!class /Script/Engine.MaterialInstanceDynamic)
      (Rendering|Material|SetMaterial _array_element 0 _returnvalue_2))))

(event Custom|Unhighlight
  (if (Variables|Default|GetHighlighted)
    (Variables|Default|SetHighlighted false)
    (for _array_element (CallFunction|GetHighlightables)
      (bind _returnvalue (Rendering|Material|GetBaseMaterial (Rendering|Material|GetMaterial _array_element 0)))
      (bind _returnvalue_2 (Rendering|Material|CreateDynamicMaterialInstance _returnvalue "None" :!class /Script/Engine.KismetMaterialLibrary))
      (Rendering|Material|SetScalarParameterValue _returnvalue_2 "Highlight" 0.0 :!class /Script/Engine.MaterialInstanceDynamic)
      (Rendering|Material|SetMaterial _array_element 0 _returnvalue_2))))

(event EventBeginPlay
  (Rendering|SceneCapture|ShowOnlyActorComponents (Variables|Default|GetCapture) self true))

(event EventTick
  (params (DeltaSeconds :type Float%20%28single-precision%29))
  (for _array_element (Actor|GetComponentsByClass "/Game/Logic/Blueprints/Snap.Snap_C")
    (for _array_element_2 (Variables|/Game/Logic/Blueprints/Snap.Snap_C|GetAllowedComponents _array_element)
      (if (== _array_element_2 (Variables|/Game/Logic/Blueprints/GM.GM_C|GetShowSnapsFor (Utilities|GetGM)))
        (Rendering|SetVisibility _array_element true false)
        (else
          (Rendering|SetVisibility _array_element false false))))))

(fn ConstructionScript)

(fn GetHighlightables
  (return 0))