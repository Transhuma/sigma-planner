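; UserSettings is an actor Blueprint that holds and persists the user's settings and canceled tips.
; On BeginPlay it loads a UserSettingsStorage save object from its storage slot, or creates a new one if none exists, then copies Settings and CanceledTips into its own variables.
; Its SaveGame event writes both variables back to the storage object and saves it to the same slot.
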(event Custom|SaveGame
  (bind _storage (Variables|Default|GetStorage))
  (Variables|/Game/Logic/Blueprints/UserSettingsStorage.UserSettingsStorage_C|SetSettings _storage (Variables|Default|GetSettings))
  (Variables|/Game/Logic/Blueprints/UserSettingsStorage.UserSettingsStorage_C|SetCanceledTips _storage (Variables|Default|GetCanceledTips))
  (SaveGame|SaveGametoSlot (Variables|Default|GetStorage) (Variables|Default|GetStorageSlot)))

(event EventBeginPlay
  (bind _storageslot (Variables|Default|GetStorageSlot))
  (bind _returnvalue (SaveGame|DoesSaveGameExist _storageslot))
  (if _returnvalue
    (bind _returnvalue_2 (SaveGame|LoadGamefromSlot _storageslot))
    (bind _output_get (Variables|Default|SetStorage (.AsUser%20Settings%20Storage (Utilities|Casting|CastToUserSettingsStorage _returnvalue_2))))
    (Variables|Default|SetSettings (Variables|/Game/Logic/Blueprints/UserSettingsStorage.UserSettingsStorage_C|GetSettings _output_get))
    (Variables|Default|SetCanceledTips (Variables|/Game/Logic/Blueprints/UserSettingsStorage.UserSettingsStorage_C|GetCanceledTips _output_get))
    (else
      (bind _returnvalue_3 (SaveGame|CreateSaveGameObject "/Game/Logic/Blueprints/UserSettingsStorage.UserSettingsStorage_C"))
      (bind _output_get_2 (Variables|Default|SetStorage _returnvalue_3))
      (Variables|Default|SetSettings (Variables|/Game/Logic/Blueprints/UserSettingsStorage.UserSettingsStorage_C|GetSettings _output_get_2))
      (Variables|Default|SetCanceledTips (Variables|/Game/Logic/Blueprints/UserSettingsStorage.UserSettingsStorage_C|GetCanceledTips _output_get_2)))))

(fn ConstructionScript)