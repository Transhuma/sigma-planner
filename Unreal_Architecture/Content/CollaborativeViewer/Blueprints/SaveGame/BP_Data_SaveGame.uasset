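; BP_Data_SaveGame is a save-game data Blueprint for the Collaborative Viewer, holding transformed actor, X-ray and annotation state.
; It keeps arrays of transformed actors with their names and transforms, X-rayed actors with their names, and annotation point transforms and last indices.
; ClearSaveGameArrays empties all of these arrays in one call.
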(fn ClearSaveGameArrays
  (Utilities|Array|Clear (Variables|Default|GetTransformedAcrors))
  (Utilities|Array|Clear (Variables|Default|GetActorTransform))
  (Utilities|Array|Clear (Variables|Default|GetXrayActors))
  (Utilities|Array|Clear (Variables|Default|GetXrayObjectNames))
  (Utilities|Array|Clear (Variables|Default|GetTransformedObjectNames))
  (Utilities|Array|Clear (Variables|Default|GetAnnotationPointTransform))
  (Utilities|Array|Clear (Variables|Default|GetAnnotationLastIndex)))