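; Explode command component for the Collaborative Viewer that adds an "Explode" option button to play the explode animation on scene actors.
; Gathers all BP_Explode actors at BeginPlay and binds the button after pawn spawn.
; On press, sends each actor through the local pawn's Explode component, where StartAnim_ROS relays to StartAnim_MTC (server-to-multicast, by naming) to call ExplodeAnim.
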(event Custom|Option1
  ;[0.3384 0.6313 1] Setup Option Buttons
  (bind _asbp_base_pawn (Utilities|Casting|CastToBP_BasePawn (Game|Player|GetPlayerPawn 0)))
  (for _array_element (Variables|Default|GetExplodeData)
    (CallFunction|StartAnimROS (Variables|/Game/CollaborativeViewer/Blueprints/Pawn/BP_BasePawn.BP_BasePawn_C|GetExplode _asbp_base_pawn) _array_element)))

(event Custom|StartAnim_ROS
  (params (ExplodeActor :type BP%20Explode%20Object%20Reference))
  ;[0.3384 0.6313 1] Animation
  (CallFunction|StartAnimMTC ExplodeActor))

(event Custom|StartAnim_MTC
  (params (ExplodeActor :type BP%20Explode%20Object%20Reference))
  ;[0.3384 0.6313 1] Animation
  (Default|ExplodeAnim ExplodeActor))

(event Custom|Bind_Option_Desktop
  (bind _optionsbuttons (Variables|Default|GetOptionsButtons))
  (bind _output (Utilities|Array|Get(acopy) _optionsbuttons))
  ;[0.3384 0.6313 1] Setup Option Buttons
  (Variables|/Game/CollaborativeViewer/UMG/GameMenu/Option_Button.Option_Button_C|SetWhenExecute _output "NewEnumerator1")
  (EventDispatchers|BindEventtoOnReleased (Variables|/Game/CollaborativeViewer/UMG/GameMenu/Base_Button.Base_Button_C|GetButton _output) (delegate Custom|Option1))
  (EventDispatchers|BindEventtoExecute _output (delegate Custom|Option1)))

(event EventBeginPlay
  ;[0 1 0.1488] BeginPlayAfterSpawn
  (bind _outactors (Actor|GetAllActorsOfClass "/Game/CollaborativeViewer/Blueprints/Commands/Explode/BP_Explode.BP_Explode_C"))
  (Variables|Default|SetExplodeData _outactors))

(event EventExecuteAfterSpawnPawn
  ;[0 1 0.1488] BeginPlayAfterSpawn
  (Variables|Default|SetOptionsButtonNames (Utilities|Array|MakeArray "Explode"))
  (Variables|Default|SetName "Explode")
  (CallFunction|CreateContextualButon)
  (CallFunction|BindOptionDesktop))