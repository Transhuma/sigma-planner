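; Player pawn for the Architectual Construct system, providing free movement and stepped rotation.
; WalkForward, WalkRight and FlyUp axes add movement input along the Sphere component's forward, right and up vectors.
; SpinRight and SpinLeft use timelines to lerp Sphere yaw from its current value toward the starting yaw offset by RotationAmmount, zeroing pitch and roll.
; R calls MouseToggle on the Architectual_Controller cached at BeginPlay.
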(event EventBeginPlay
  ;[1 1 1] References
  (bind _asarchitectual_controller (Utilities|Casting|CastToArchitectual_Controller (Pawn|GetController self)))
  (Variables|Default|SetController_REF _asarchitectual_controller))

(event Input|ActionEvents|InputActionSpinLeft
  (params (Key :type Key%20Structure :default "None"))
  (bind _sphere (Variables|Default|GetSphere))
  (bind _returnvalue (Transformation|GetWorldRotation _sphere))
  ;[1 1 1] Rotation
  (:Pressed
    (bind _output_get (Variables|Default|SetWorld_Rotation (.yaw _returnvalue)))
    (bind _lerp (Timeline|Timeline_1 PlayFromStart)
      (:Update
        (Transformation|SetWorldRotation _sphere (Math|Rotator|MakeRotator 0.0 0.0 (Math|Float|Lerp (.yaw _returnvalue) (- _output_get (Variables|Default|GetRotation_Ammount)) _lerp)) false false)))))

(event Input|ActionEvents|InputActionSpinRight
  (params (Key :type Key%20Structure :default "None"))
  (bind _sphere (Variables|Default|GetSphere))
  (bind _returnvalue (Transformation|GetWorldRotation _sphere))
  ;[1 1 1] Rotation
  (:Pressed
    (bind _output_get (Variables|Default|SetWorld_Rotation (.yaw _returnvalue)))
    (bind _lerp (Timeline|Timeline_0 PlayFromStart)
      (:Update
        (Transformation|SetWorldRotation _sphere (Math|Rotator|MakeRotator 0.0 0.0 (Math|Float|Lerp (.yaw _returnvalue) (+ _output_get (Variables|Default|GetRotation_Ammount)) _lerp)) false false)))))

(event Input|AxisEvents|InputAxisWalkForward
  (params (AxisValue :type Float%20%28single-precision%29))
  ;[1 1 1] Movement
  (Pawn|Input|AddMovementInput (Math|Vector|GetForwardVector (Variables|Default|GetSphere)) AxisValue false))

(event Input|AxisEvents|InputAxisWalkRight
  (params (AxisValue :type Float%20%28single-precision%29))
  ;[1 1 1] Movement
  (Pawn|Input|AddMovementInput (Math|Vector|GetRightVector (Variables|Default|GetSphere)) AxisValue false))

(event Input|AxisEvents|InputAxisFlyUp
  (params (AxisValue :type Float%20%28single-precision%29))
  ;[1 1 1] Movement
  (Pawn|Input|AddMovementInput (Math|Vector|GetUpVector (Variables|Default|GetSphere)) AxisValue false))

(event Input|KeyboardEvents|R
  (params (Key :type Key%20Structure :default "None"))
  ;[1 1 1] Mouse Toggle
  (:Pressed
    (Default|MouseToggle (Variables|Default|GetController_REF))))

(fn ConstructionScript)