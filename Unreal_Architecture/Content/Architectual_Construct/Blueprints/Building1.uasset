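; Building1 is a modular building piece that grows through clickable spawn and extend controls.
; On BeginPlay it snaps both control sets to four static mesh sockets and hides them, appending extenders to the spawn array.
; Hovering over the Cube reveals that array, which hides again shortly after the cursor leaves.
; Spawn clicks create another Building1 at that socket, while Extend clicks swap and rotate the mesh, then re-snap the controls.
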(event OnClicked(Extend1)
  (params (TouchedComponent :type Primitive%20Component%20Object%20Reference) (ButtonPressed :type Key%20Structure :default "None"))
  (bind _staticmesh (Variables|Default|GetStaticMesh))
  (Components|StaticMesh|SetStaticMesh _staticmesh "/Game/Architectual_Construct/Mesh_Components/2.2")
  (Transformation|SetRelativeRotation _staticmesh "0,90.000000, 0" false false)
  (CallFunction|SetTransforms)
  (Development|PrintString "Hello"))

(event OnClicked(Extend2)
  (params (TouchedComponent :type Primitive%20Component%20Object%20Reference) (ButtonPressed :type Key%20Structure :default "None"))
  (bind _staticmesh (Variables|Default|GetStaticMesh))
  (Components|StaticMesh|SetStaticMesh _staticmesh "/Game/Architectual_Construct/Mesh_Components/2.2")
  (Transformation|SetRelativeRotation _staticmesh "0,-90.000000, 0" false false)
  (CallFunction|SetTransforms)
  (Development|PrintString "Hello"))

(event OnClicked(Extend3)
  (params (TouchedComponent :type Primitive%20Component%20Object%20Reference) (ButtonPressed :type Key%20Structure :default "None"))
  (bind _staticmesh (Variables|Default|GetStaticMesh))
  (Components|StaticMesh|SetStaticMesh _staticmesh "/Game/Architectual_Construct/Mesh_Components/2.2")
  (Transformation|SetRelativeRotation _staticmesh "0,180.000000, 0" false false)
  (CallFunction|SetTransforms)
  (Development|PrintString "Hello"))

(event OnClicked(Spawn1)
  (params (TouchedComponent :type Primitive%20Component%20Object%20Reference) (ButtonPressed :type Key%20Structure :default "None"))
  (Game|SpawnActorfromClass "Building1_C" (Transformation|GetWorldTransform TouchedComponent) "Undefined" 0 0))

(event OnClicked(Spawn2)
  (params (TouchedComponent :type Primitive%20Component%20Object%20Reference) (ButtonPressed :type Key%20Structure :default "None"))
  (Game|SpawnActorfromClass "Building1_C" (Transformation|GetWorldTransform TouchedComponent) "Undefined" 0 0))

(event OnBeginCursorOver(Cube)
  (params (TouchedComponent :type Primitive%20Component%20Object%20Reference))
  (for _array_element (Variables|Default|GetSpawns)
    (Development|SetHiddeninGame _array_element false false)))

(event OnEndCursorOver(Cube)
  (params (TouchedComponent :type Primitive%20Component%20Object%20Reference))
  (Utilities|FlowControl|Delay 2.0)
  (for _array_element (Variables|Default|GetSpawns)
    (Development|SetHiddeninGame _array_element true false)))

(event OnClicked(Spawn3)
  (params (TouchedComponent :type Primitive%20Component%20Object%20Reference) (ButtonPressed :type Key%20Structure :default "None"))
  (Game|SpawnActorfromClass "Building1_C" (Transformation|GetWorldTransform TouchedComponent) "Undefined" 0 0))

(event OnClicked(Spawn4)
  (params (TouchedComponent :type Primitive%20Component%20Object%20Reference) (ButtonPressed :type Key%20Structure :default "None"))
  (Game|SpawnActorfromClass "Building1_C" (Transformation|GetWorldTransform TouchedComponent) "Undefined" 0 0))

(event OnClicked(Extend4)
  (params (TouchedComponent :type Primitive%20Component%20Object%20Reference) (ButtonPressed :type Key%20Structure :default "None"))
  (bind _staticmesh (Variables|Default|GetStaticMesh))
  (Components|StaticMesh|SetStaticMesh _staticmesh "/Game/Architectual_Construct/Mesh_Components/2.2")
  (Transformation|SetRelativeRotation _staticmesh "0,0.000000, 0" false false)
  (CallFunction|SetTransforms)
  (Development|PrintString "Hello"))

(event Custom|Set_Transforms
  (bind _newparam (CallFunction|GetSocketLocations))
  (for (_array_element _array_index) (Variables|Default|GetSpawns)
    (Transformation|SetRelativeTransform _array_element (Utilities|Array|Get(acopy) _newparam _array_index) false false)
    (Development|SetHiddeninGame _array_element true false))
  (for (_array_element_2 _array_index_2) (Variables|Default|GetExtenders)
    (Transformation|SetRelativeTransform _array_element_2 (Utilities|Array|Get(acopy) _newparam _array_index_2) false false)
    (Development|SetHiddeninGame _array_element_2 true false)
    (Utilities|Array|AppendArray (Variables|Default|GetSpawns) (Variables|Default|GetExtenders))))

(event EventBeginPlay
  (bind _extenders (Variables|Default|GetExtenders))
  (bind _spawns (Variables|Default|GetSpawns))
  (Utilities|Array|Add _spawns (Variables|Default|GetSpawn1))
  (Utilities|Array|Add _spawns (Variables|Default|GetSpawn2))
  (Utilities|Array|Add _spawns (Variables|Default|GetSpawn3))
  (Utilities|Array|Add _spawns (Variables|Default|GetSpawn4))
  (Utilities|Array|Add _extenders (Variables|Default|GetExtend1))
  (Utilities|Array|Add _extenders (Variables|Default|GetExtend2))
  (Utilities|Array|Add _extenders (Variables|Default|GetExtend3))
  (Utilities|Array|Add _extenders (Variables|Default|GetExtend4))
  (CallFunction|SetTransforms))

(fn ConstructionScript)

(fn GetSocketLocations
  (bind _staticmesh (Variables|Default|GetStaticMesh))
  (bind _socket_transforms (Variables|Default|GetSocket_Transforms))
  (Utilities|Array|Add _socket_transforms (Transformation|GetSocketTransform _staticmesh "1" "RTS_Component"))
  (Utilities|Array|Add _socket_transforms (Transformation|GetSocketTransform _staticmesh "2" "RTS_Component"))
  (Utilities|Array|Add _socket_transforms (Transformation|GetSocketTransform _staticmesh "3" "RTS_Component"))
  (Utilities|Array|Add _socket_transforms (Transformation|GetSocketTransform _staticmesh "4" "RTS_Component"))
  (return _socket_transforms "" "" "" ""))

(fn AddControlComponents
  (params (NewParam :type Array%20of%20Transforms))
  (bind _spawn1 (Variables|Default|GetSpawn1))
  (for _array_element NewParam
    (Transformation|SetRelativeTransform _spawn1 _array_element false false)
    (Development|SetHiddeninGame _spawn1 true false)
    (Utilities|Array|Add (Variables|Default|GetSpawns) 0))
  (for _array_element_2 NewParam
    _))