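; Building_BP1 is a modular building block actor that the player extends by clicking on it to spawn more copies of itself.
; Each of five cube components handles OnClicked and spawns a new Building_BP1 offset from the root's world location along plus or minus X, plus or minus Y, or upward in Z.
; Spawning always ignores collisions, and the graph has no check for an already occupied spot.
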(event OnClicked(Cube5)
  (params (TouchedComponent :type Primitive%20Component%20Object%20Reference) (ButtonPressed :type Key%20Structure :default "None"))
  (bind _defaultsceneroot (Variables|Default|GetDefaultSceneRoot))
  (bind _returnvalue (Transformation|GetWorldLocation _defaultsceneroot))
  (Game|SpawnActorfromClass "Building_BP1_C" (Math|Transform|MakeTransform (Math|Vector|MakeVector (.x _returnvalue) (.y _returnvalue) (+ (.z _returnvalue) 245.0)) "0, 0, 0" "1,1,1") "AlwaysSpawn" 0 0))

(event OnClicked(Cube4)
  (params (TouchedComponent :type Primitive%20Component%20Object%20Reference) (ButtonPressed :type Key%20Structure :default "None"))
  (bind _defaultsceneroot (Variables|Default|GetDefaultSceneRoot))
  (bind _returnvalue (Transformation|GetWorldLocation _defaultsceneroot))
  (Game|SpawnActorfromClass "Building_BP1_C" (Math|Transform|MakeTransform (Math|Vector|MakeVector (.x _returnvalue) (+ (.y _returnvalue) 2.9e+02) (.z _returnvalue)) "0, 0, 0" "1,1,1") "AlwaysSpawn" 0 0))

(event OnClicked(Cube1)
  (params (TouchedComponent :type Primitive%20Component%20Object%20Reference) (ButtonPressed :type Key%20Structure :default "None"))
  (bind _defaultsceneroot (Variables|Default|GetDefaultSceneRoot))
  (bind _returnvalue (Transformation|GetWorldLocation _defaultsceneroot))
  (Game|SpawnActorfromClass "Building_BP1_C" (Math|Transform|MakeTransform (Math|Vector|MakeVector (+ (.x _returnvalue) 2.9e+02) (.y _returnvalue) (.z _returnvalue)) "0, 0, 0" "1,1,1") "AlwaysSpawn" 0 0))

(event OnClicked(Cube2)
  (params (TouchedComponent :type Primitive%20Component%20Object%20Reference) (ButtonPressed :type Key%20Structure :default "None"))
  (bind _defaultsceneroot (Variables|Default|GetDefaultSceneRoot))
  (bind _returnvalue (Transformation|GetWorldLocation _defaultsceneroot))
  (Game|SpawnActorfromClass "Building_BP1_C" (Math|Transform|MakeTransform (Math|Vector|MakeVector (+ (.x _returnvalue) -2.9e+02) (.y _returnvalue) (.z _returnvalue)) "0, 0, 0" "1,1,1") "AlwaysSpawn" 0 0))

(event OnClicked(Cube3)
  (params (TouchedComponent :type Primitive%20Component%20Object%20Reference) (ButtonPressed :type Key%20Structure :default "None"))
  (bind _defaultsceneroot (Variables|Default|GetDefaultSceneRoot))
  (bind _returnvalue (Transformation|GetWorldLocation _defaultsceneroot))
  (Game|SpawnActorfromClass "Building_BP1_C" (Math|Transform|MakeTransform (Math|Vector|MakeVector (.x _returnvalue) (+ (.y _returnvalue) -2.9e+02) (.z _returnvalue)) "0, 0, 0" "1,1,1") "AlwaysSpawn" 0 0))

(fn ConstructionScript)